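; Dialogue NPC "happygirl" that offers a conversation with a choice awarding the player light or dark points.
; After conversation setup it queues an opening line, and its dialogue-end handler adds a three-option decision.
; The decision handler maps option indices to increments of the player's LightPoints or DarkPoints, prints a message and ends the conversation.
; Line and option texts appear to be placeholders.
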(event `self.AfterConversationSetup`
  (`self.AddCustomImportantDialogue` 0 (make `/Game/DialogueSystem/Blueprints/Structures/s_DialogueInfo` null "First chat")))

(event `self.OnDialogueEnd`
  (params (Index :type Integer))
  (switch `int` Index
    (:`Default`
      (`self.AddDecision` 0 (make `/Game/DialogueSystem/Blueprints/Structures/s_DecisionInfo` (make `/Game/DialogueSystem/Blueprints/Structures/s_DialogueInfo` null "various options") (`|MakeArray` (make `/Game/DialogueSystem/Blueprints/Structures/s_OptionInfo` "First") (make `/Game/DialogueSystem/Blueprints/Structures/s_OptionInfo` "Second") (make `/Game/DialogueSystem/Blueprints/Structures/s_OptionInfo` "Third") :!type "/Game/DialogueSystem/Blueprints/Structures/s_OptionInfo Structure"))))))

(event `self.OnDecisionMade`
  (params (DecisionIndex :type Integer) (ChosenOptionIndex :type Integer))
  (bind _playerchar (`self.PlayerChar`))
  ;[1 1 1] this is where yo uchoose what happens after you choose each option
  (switch `int` DecisionIndex
    (:`0`
      (switch `int` ChosenOptionIndex
        (:`1`
          ;[1 1 1] This is supposed to give points for each choice
          (set `/Game/ThirdPersonBP/Blueprints/ThirdPersonCharacter.LightPoints` (+ (`/Game/ThirdPersonBP/Blueprints/ThirdPersonCharacter.LightPoints` _playerchar) 1) _playerchar :!label _label)
          (`KismetSystemLibrary.PrintString` "You get point A"))
        (:`2`
          (goto _label))
        (:`3`
          (set `/Game/ThirdPersonBP/Blueprints/ThirdPersonCharacter.DarkPoints` (+ (`/Game/ThirdPersonBP/Blueprints/ThirdPersonCharacter.DarkPoints` _playerchar) 1) _playerchar)
          (`KismetSystemLibrary.PrintString` "You get point B")))
      (`self.EndConversation`))))

(fn `UserConstructionScript`
  (`parent.UserConstructionScript`))